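; AI controller for the cat that sets up its blackboard and runs the BT_LeavingCat behavior tree.
; Setup runs once on the first Tick rather than BeginPlay, writing the player pawn, the Runorstop flag and Mixamo_Maria's capsule location to BB_Cat.
; The target location is a one-time snapshot, and a failed player cast prevents the tree from starting.
; SetBehaviorTree runs any tree passed to it.
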(event EventBeginPlay)

(event EventTick
  (params (DeltaSeconds :type Float%20%28single-precision%29))
  (Utilities|FlowControl|Sequence
    (:then_0
      (Utilities|FlowControl|DoOnce false
        (:Completed
          (bind _blackboardcomponent (Class|AIController|UseBlackboard "/Game/Game/Character/AI/BB_Cat.BB_Cat"))
          (AI|Components|Blackboard|SetValueasObject _blackboardcomponent (Variables|Default|GetTargetActor) (Game|Player|GetPlayerPawn 0))
          (AI|Components|Blackboard|SetValueasBool _blackboardcomponent (Variables|Default|GetState) (Variables|Default|Getrunorstop))
          (bind _asmixamo_maria (Utilities|Casting|CastToMixamo_Maria (Game|Player|GetPlayerPawn 0)))
          (AI|Components|Blackboard|SetValueasVector _blackboardcomponent (Variables|Default|GetTargetloc) (Transformation|GetWorldLocation (Variables|/Script/Engine.Character|GetCapsuleComponent _asmixamo_maria)))
          (AI|RunBehaviorTree "/Game/Game/Character/AI/BT_LeavingCat.BT_LeavingCat"))))))

(fn ConstructionScript)

(fn SetBehaviorTree
  (params (BehaviorTree :type Behavior%20Tree%20Object%20Reference))
  (AI|RunBehaviorTree BehaviorTree))