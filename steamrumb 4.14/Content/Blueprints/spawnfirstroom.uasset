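; Room spawner actor that spawns AIchara pawns running BT_LeavingCat and ends the first floor's wave.
; Tick counts frames up to an interval, then spawns at one of four randomly chosen locations and shortens the interval, so spawns speed up.
; Once the interval drops below 250, it waits briefly, sets Floorclear1 on stiranGameState and destroys itself.
; Spawn branches for AIchara2 and AILongverchara are left unconnected.
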(event EventBeginPlay)

(event Collision|EventActorBeginOverlap
  (params (OtherActor :type Actor%20Object%20Reference)))

(event EventTick
  (params (DeltaSeconds :type Float%20%28single-precision%29))
  (if (< (Variables|Default|GetNewVar_8) 250)
    (Utilities|FlowControl|DoOnce false
      (:Completed
        (Utilities|FlowControl|Delay 5.0)
        (Variables|/Game/Blueprints/stiranGameState.stiranGameState_C|Setfloorclear1 (.AsStiran%20Game%20State (Utilities|Casting|CastTostiranGameState (Game|GetGameState))) true)
        (Actor|DestroyActor)))
    (else
      (bind _output_get (Variables|Default|Setcount (+ (Variables|Default|Getcount) 1)))
      (if (> _output_get (Variables|Default|GetNewVar_8))
        (bind _output_get_2 (Variables|Default|SetNewVar_6 (Math|Random|RandomInteger 4)))
        (if (== _output_get_2 0)
          (Variables|Default|SetNewVar_5 (Variables|Default|GetNewVar_1))
          (elif (== _output_get_2 1)
            (Variables|Default|SetNewVar_5 (Variables|Default|GetNewVar_2))
            (elif (== _output_get_2 2)
              (Variables|Default|SetNewVar_5 (Variables|Default|GetNewVar_3))
              (else
                (Variables|Default|SetNewVar_5 (Variables|Default|GetNewVar_4))))))
        (AI|SpawnAIFromClass "/Game/TopDownBP/Blueprints/AIchara.AIchara_C" "/Game/Game/Character/AI/BT_LeavingCat.BT_LeavingCat" (Variables|Default|GetNewVar_5) "0, 0, 0" false)
        (Variables|Default|Setcount 0)
        (Variables|Default|SetNewVar_8 (Math|Integer|Max(Integer) (- (Variables|Default|GetNewVar_8) 10) 200))))))

(fn ConstructionScript)