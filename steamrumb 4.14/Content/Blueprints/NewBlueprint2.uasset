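; NewBlueprint2 is an actor that periodically spawns AI characters at one of four preset locations.
; Each Tick it adds a small random amount to a counter, giving an irregular, frame-rate-dependent spawn interval.
; When the counter passes a threshold, it picks one of the four locations at random, spawns the AIchara pawn with the AIT behavior tree there, and resets the counter.
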(event EventBeginPlay)

(event Collision|EventActorBeginOverlap
  (params (OtherActor :type Actor%20Object%20Reference)))

(event EventTick
  (params (DeltaSeconds :type Float%20%28single-precision%29))
  (bind _output_get (Variables|Default|Setcount (+ (Variables|Default|Getcount) (Math|Random|RandomInteger 5))))
  (if (> _output_get 2080)
    (bind _output_get_2 (Variables|Default|SetNewVar_6 (Math|Random|RandomInteger 4)))
    (if (== _output_get_2 0)
      (Variables|Default|SetNewVar_5 (Variables|Default|GetNewVar_1))
      (elif (== _output_get_2 1)
        (Variables|Default|SetNewVar_5 (Variables|Default|GetNewVar_2))
        (elif (== _output_get_2 2)
          (Variables|Default|SetNewVar_5 (Variables|Default|GetNewVar_3))
          (else
            (Variables|Default|SetNewVar_5 (Variables|Default|GetNewVar_4))))))
    (AI|SpawnAIFromClass "/Game/TopDownBP/Blueprints/AIchara.AIchara_C" "/Game/TopDownBP/Blueprints/AIT.AIT" (Variables|Default|GetNewVar_5) "0, 0, 0" false)
    (Variables|Default|Setcount 0)))

(fn ConstructionScript)