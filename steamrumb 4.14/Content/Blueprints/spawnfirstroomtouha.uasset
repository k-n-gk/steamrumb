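; Spawner actor that releases AI characters at an accelerating pace, then spawns a Goal and destroys itself.
; A Tick frame counter triggers each spawn at one of four random locations, choosing between AIchara and AILongverchara; the AIchara2 branch is unreachable.
; Each spawn shortens the interval toward a floor.
; Once it drops below the threshold, a DoOnce and delay place the Goal at a fixed position.
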(event EventBeginPlay)

(event Collision|EventActorBeginOverlap
  (params (OtherActor :type Actor%20Object%20Reference)))

(event EventTick
  (params (DeltaSeconds :type Float%20%28single-precision%29))
  (if (< (Variables|Default|GetNewVar_8) 210)
    (Utilities|FlowControl|DoOnce false
      (:Completed
        (Utilities|FlowControl|Delay 5.0)
        (Game|SpawnActorfromClass "/Game/WaterPlane/Meshes/goal.goal_C" (Math|Transform|MakeTransform "-2930.000000,1830.000000,180.000000") "Undefined" 0 0)
        (Actor|DestroyActor)))
    (else
      (bind _output_get (Variables|Default|Setcount (+ (Variables|Default|Getcount) 1)))
      (if (> _output_get (Variables|Default|GetNewVar_8))
        (bind _output_get_2 (Variables|Default|SetNewVar_6 (Math|Random|RandomInteger 4)))
        (if (== _output_get_2 0)
          (Variables|Default|SetNewVar_5 (Variables|Default|GetNewVar_1))
          (elif (== _output_get_2 1)
            (Variables|Default|SetNewVar_5 (Variables|Default|GetNewVar_2))
            (elif (== _output_get_2 2)
              (Variables|Default|SetNewVar_5 (Variables|Default|GetNewVar_3))
              (else
                (Variables|Default|SetNewVar_5 (Variables|Default|GetNewVar_4))))))
        (bind _output_get_3 (Variables|Default|SetNewVar_7 (Math|Random|RandomInteger 6)))
        (if (< _output_get_3 3)
          (AI|SpawnAIFromClass "/Game/TopDownBP/Blueprints/AIchara.AIchara_C" "/Game/Game/Character/AI/BT_LeavingCat.BT_LeavingCat" (Variables|Default|GetNewVar_5) "0, 0, 0" false)
          (elif (< _output_get_3 6)
            (AI|SpawnAIFromClass "/Game/TopDownBP/Blueprints/AILongverchara.AILongverchara_C" "/Game/Game/Character/AI/BT_Leaving2.BT_Leaving2" (Variables|Default|GetNewVar_5) "0, 0, 0" false)
            (else
              (AI|SpawnAIFromClass "/Game/TopDownBP/Blueprints/AIchara2.AIchara2_C" "/Game/Game/Character/AI/BT_LeavingCat.BT_LeavingCat" (Variables|Default|GetNewVar_5) "0,0.000000, 0" false))))
        (Variables|Default|Setcount 0)
        (Variables|Default|SetNewVar_8 (Math|Integer|Max(Integer) (- (Variables|Default|GetNewVar_8) 10) 200))))))

(fn ConstructionScript)