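; A short-lived physics part actor that kills AI characters it touches.
; On overlap, actors named with an "A" prefix are cast to AIchara and, if not already dying, ragdolled and flagged as killed by parts.
; Overlapping "tri"-prefixed actors instead push the mesh away with a strong, upward-biased impulse scaled by their offset.
; It gets a small impulse on spawn and destroys itself after a fixed tick count, so lifetime depends on frame rate.
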(event EventBeginPlay
  (Physics|AddImpulse (Variables|Default|GetStaticMesh) "0,-20.000000,1.000000" "None" false))

(event Collision|EventActorBeginOverlap
  (params (OtherActor :type Actor%20Object%20Reference))
  (bind _returnvalue (Utilities|GetDisplayName OtherActor))
  (if (Utilities|String|StartsWith _returnvalue "A")
    (bind _asaichara (Utilities|Casting|CastToAIchara OtherActor))
    (if (not (Variables|/Game/TopDownBP/Blueprints/AIchara.AIchara_C|Getdying _asaichara))
      (Physics|SetSimulatePhysics (Variables|/Script/Engine.Character|GetMesh _asaichara) true)
      (Variables|/Game/TopDownBP/Blueprints/AIchara.AIchara_C|Setpartsdead _asaichara true)
      (Variables|/Game/TopDownBP/Blueprints/AIchara.AIchara_C|Setdying _asaichara true))
    (elif (Utilities|String|StartsWith _returnvalue "tri")
      (Physics|AddImpulse (Variables|Default|GetStaticMesh) (* (- (+ (Transformation|GetWorldLocation (Variables|Default|GetStaticMesh)) "0, 0,100.000000") (Transformation|GetActorLocation OtherActor)) 2000) "None" false))))

(event EventTick
  (params (DeltaSeconds :type Float%20%28single-precision%29))
  (bind _output_get (Variables|Default|Setlifetime (+ (Variables|Default|Getlifetime) 1)))
  (if (> _output_get 1800)
    (Variables|Default|Setlifetime 0)
    (Actor|DestroyActor)))

(event Input|GamepadEvents|GamepadFaceButtonTop
  (params (Key :type Key%20Structure :default "AnyKey")))

(fn ConstructionScript)