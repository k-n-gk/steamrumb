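; Destructible debris actor that shatters on spawn through heavy self-applied damage and can kill AI characters it overlaps.
; Overlaps are sorted by display-name prefix: "A" actors cast to AIchara are ragdolled and flagged as dying, while "tri" actors knock the debris away with an upward-biased impulse.
; A per-frame Tick counter destroys the actor after a fixed number of frames, so its lifetime depends on framerate.
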(event EventBeginPlay
  (bind _destructible (Variables|Default|GetDestructible))
  (Game|Damage|ApplyDamage _destructible 1e+03 (Transformation|GetWorldLocation _destructible) (Math|Vector|MakeVector 0.0 1.0 0.0) 1e+03))

(event Collision|EventActorBeginOverlap
  (params (OtherActor :type Actor%20Object%20Reference))
  (bind _returnvalue (Utilities|GetDisplayName OtherActor))
  (bind _destructible (Variables|Default|GetDestructible))
  (if (Utilities|String|StartsWith _returnvalue "A")
    (bind _asaichara (Utilities|Casting|CastToAIchara OtherActor))
    (if (not (Variables|/Game/TopDownBP/Blueprints/AIchara.AIchara_C|Getdying _asaichara))
      (Physics|SetSimulatePhysics (Variables|/Script/Engine.Character|GetMesh _asaichara) true)
      (Variables|/Game/TopDownBP/Blueprints/AIchara.AIchara_C|Setpartsdead _asaichara true)
      (Variables|/Game/TopDownBP/Blueprints/AIchara.AIchara_C|Setdying _asaichara true))
    (elif (Utilities|String|StartsWith _returnvalue "tri")
      (Physics|AddImpulse _destructible (* (- (+ (Transformation|GetWorldLocation _destructible) "0, 0,100.000000") (Transformation|GetActorLocation OtherActor)) 2000) "None" false))))

(event EventTick
  (params (DeltaSeconds :type Float%20%28single-precision%29))
  (bind _output_get (Variables|Default|Setlifetime (+ (Variables|Default|Getlifetime) 1)))
  (if (> _output_get 1800)
    (Variables|Default|Setlifetime 0)
    (Actor|DestroyActor)))

(event Input|GamepadEvents|GamepadFaceButtonTop
  (params (Key :type Key%20Structure :default "AnyKey")))

(fn ConstructionScript)