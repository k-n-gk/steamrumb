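; Destructible debris actor that shatters on spawn and can be struck by the player to set off an explosion.
; BeginPlay applies damage and an impulse to its Destructible component.
; Each Tick, an overlapping Mixamo_Maria pawn with Atking set in stiranPlayerState makes it spawn a Triggerbomb, play a sound, clear the flag and destroy itself.
; Otherwise a frame-based counter destroys it after a fixed lifetime.
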(event EventBeginPlay
  (bind _destructible (Variables|Default|GetDestructible))
  (Game|Damage|ApplyDamage _destructible 1e+03 (Transformation|GetWorldLocation _destructible) (Math|Vector|MakeVector 0.0 1.0 0.0) 1e+03))

(event Collision|EventActorBeginOverlap
  (params (OtherActor :type Actor%20Object%20Reference)))

(event EventTick
  (params (DeltaSeconds :type Float%20%28single-precision%29))
  (bind _returnvalue (Game|Player|GetPlayerPawn 0))
  (bind _destructible (Variables|Default|GetDestructible))
  (bind _returnvalue_2 (Transformation|GetWorldLocation _destructible))
  (bind _playerstate (Variables|/Script/Engine.Pawn|GetPlayerState _returnvalue))
  (bind (_x _y) (Math|Vector|BreakVector _returnvalue_2))
  (bind _asstiran_player_state (Utilities|Casting|CastTostiranPlayerState _playerstate))
  (Utilities|Casting|CastToMixamo_Maria _returnvalue
    (:then
      (if (and (Collision|IsOverlappingActor _returnvalue :!class /Script/Engine.Actor) (Variables|/Game/Blueprints/stiranPlayerState.stiranPlayerState_C|Getatking _asstiran_player_state))
        (Game|SpawnActorfromClass "/Game/Blueprints/triggerbomb.triggerbomb_C" (Math|Conversions|ToTransform(Vector) (Math|Vector|MakeVector _x _y 1e+02)) "Undefined" 0 0)
        (Audio|PlaySoundatLocation "/Game/StarterContent/Audio/Explosion02.Explosion02" _returnvalue_2)
        (Variables|/Game/Blueprints/stiranPlayerState.stiranPlayerState_C|Setatking _asstiran_player_state false)
        (Actor|DestroyActor :!label _label)
        (else
          (bind _output_get (Variables|Default|Setlifetime (+ (Variables|Default|Getlifetime) 1) :!label _label_2))
          (if (> _output_get 1800)
            (Variables|Default|Setlifetime 0)
            (goto _label)))))
    (:CastFailed
      (goto _label_2))))

(event Input|GamepadEvents|GamepadFaceButtonTop
  (params (Key :type Key%20Structure :default "AnyKey")))

(fn ConstructionScript)